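; Blueprint function library that saves and loads player, quest, drop, statue, altar and barrier data through BP_GameMode.
; Each function casts the game mode, writing to its OutSavingObject and reading from its separate SavingObject.
; Loads key player data by controller UserName, quests by owner and component name, and other data by actor object name.
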(fn `LoadAltarData`
  (params (Actor :type "Actor Object Reference"))
  (returns (`Drop data` :type "/Game/Blueprints/Struct_AltarData Structure"))
  (bind _asbp_game_mode (cast `/Game/Player/BP_GameMode` (`GameplayStatics.GetGameMode` Actor)))
  (bind _altar_data (`/Game/Blueprints/BP_SaveGame.LoadAltarData` (`/Game/Player/BP_GameMode.SavingObject` _asbp_game_mode) (`KismetSystemLibrary.GetObjectName` Actor)))
  (return _altar_data))

(fn `LoadBarrierData`
  (params (Actor :type "Actor Object Reference"))
  (returns (`Barrier data` :type "/Game/Blueprints/Struct_BarrierData Structure"))
  (bind _asbp_game_mode (cast `/Game/Player/BP_GameMode` (`GameplayStatics.GetGameMode` Actor)))
  (bind _barrrier_data (`/Game/Blueprints/BP_SaveGame.LoadBarrierData` (`/Game/Player/BP_GameMode.SavingObject` _asbp_game_mode) (`KismetSystemLibrary.GetObjectName` Actor)))
  (return _barrrier_data))

(fn `LoadDropData`
  (params (Actor :type "Actor Object Reference"))
  (returns (`Drop data` :type "/Game/Blueprints/Struct_DropItemData Structure"))
  (bind _asbp_game_mode (cast `/Game/Player/BP_GameMode` (`GameplayStatics.GetGameMode` Actor)))
  (bind _dropdata (`/Game/Blueprints/BP_SaveGame.LoadDropData` (`/Game/Player/BP_GameMode.SavingObject` _asbp_game_mode) (`KismetSystemLibrary.GetObjectName` Actor)))
  (return _dropdata))

(fn `LoadPlayerData`
  (params (Actor :type "Actor Object Reference"))
  (returns (`Player data` :type "/Game/Blueprints/Struct_PlayerData Structure"))
  (bind _asbp_player_controller (cast `/Game/Player/BP_PlayerController` Actor))
  (bind _asbp_game_mode (cast `/Game/Player/BP_GameMode` (`GameplayStatics.GetGameMode` Actor)))
  (bind _player_data (`/Game/Blueprints/BP_SaveGame.LoadPlayerData` (`/Game/Player/BP_GameMode.SavingObject` _asbp_game_mode) (`/Game/Player/BP_PlayerController.UserName` _asbp_player_controller)))
  (return _player_data))

(fn `LoadQuestData`
  (params (Component :type "ActorComponent Object Reference"))
  (returns (`Quest data` :type "/Game/Blueprints/Struct_QuestData Structure"))
  (bind _asbp_game_mode (cast `/Game/Player/BP_GameMode` (`GameplayStatics.GetGameMode` Component)))
  (bind _quest_data (`/Game/Blueprints/BP_SaveGame.LoadQuestData` (`/Game/Player/BP_GameMode.SavingObject` _asbp_game_mode) (`KismetStringLibrary.Concat_StrStr` (`KismetSystemLibrary.GetObjectName` (`ActorComponent.GetOwner` Component)) "_" (`KismetSystemLibrary.GetObjectName` Component))))
  (return _quest_data))

(fn `LoadStatueData`
  (params (Actor :type "Actor Object Reference"))
  (returns (`Drop data` :type "/Game/Blueprints/Struct_StatueData Structure"))
  (bind _asbp_game_mode (cast `/Game/Player/BP_GameMode` (`GameplayStatics.GetGameMode` Actor)))
  (bind _statue_data (`/Game/Blueprints/BP_SaveGame.LoadStatueData` (`/Game/Player/BP_GameMode.SavingObject` _asbp_game_mode) (`KismetSystemLibrary.GetObjectName` Actor)))
  (return _statue_data))

(fn `SaveAltarData`
  (params (Data :type "/Game/Blueprints/Struct_AltarData Structure") (Actor :type "Actor Object Reference"))
  (bind _asbp_game_mode (cast `/Game/Player/BP_GameMode` (`GameplayStatics.GetGameMode` Actor)))
  (`/Game/Blueprints/BP_SaveGame.SaveAltarData` (`/Game/Player/BP_GameMode.OutSavingObject` _asbp_game_mode) Data))

(fn `SaveBarierData`
  (params (Data :type "/Game/Blueprints/Struct_BarrierData Structure") (Actor :type "Actor Object Reference"))
  (bind _asbp_game_mode (cast `/Game/Player/BP_GameMode` (`GameplayStatics.GetGameMode` Actor)))
  (`/Game/Blueprints/BP_SaveGame.SaveBarrierData` (`/Game/Player/BP_GameMode.OutSavingObject` _asbp_game_mode) Data))

(fn `SaveDropData`
  (params (Data :type "/Game/Blueprints/Struct_DropItemData Structure") (Actor :type "Actor Object Reference"))
  (bind _asbp_game_mode (cast `/Game/Player/BP_GameMode` (`GameplayStatics.GetGameMode` Actor)))
  (`/Game/Blueprints/BP_SaveGame.SaveDropData` (`/Game/Player/BP_GameMode.OutSavingObject` _asbp_game_mode) Data))

(fn `SavePlayerData`
  (params (Data :type "/Game/Blueprints/Struct_PlayerData Structure") (Actor :type "Actor Object Reference"))
  (bind _asbp_game_mode (cast `/Game/Player/BP_GameMode` (`GameplayStatics.GetGameMode` Actor)))
  (`/Game/Blueprints/BP_SaveGame.SavePlayerData` (`/Game/Player/BP_GameMode.OutSavingObject` _asbp_game_mode) Data))

(fn `SaveQuestData`
  (params (Data :type "/Game/Blueprints/Struct_QuestData Structure") (Actor :type "Actor Object Reference"))
  (bind _asbp_game_mode (cast `/Game/Player/BP_GameMode` (`GameplayStatics.GetGameMode` Actor)))
  (`/Game/Blueprints/BP_SaveGame.SaveQuestData` (`/Game/Player/BP_GameMode.OutSavingObject` _asbp_game_mode) Data))

(fn `SaveStatueData`
  (params (Data :type "/Game/Blueprints/Struct_StatueData Structure") (Actor :type "Actor Object Reference"))
  (bind _asbp_game_mode (cast `/Game/Player/BP_GameMode` (`GameplayStatics.GetGameMode` Actor)))
  (`/Game/Blueprints/BP_SaveGame.SaveStatueData` (`/Game/Player/BP_GameMode.OutSavingObject` _asbp_game_mode) Data))