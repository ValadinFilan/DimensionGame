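; Quest component that steps each player controller through an ordered Quests array.
; A Players map stores each controller's quest index, and AddQuest gives the first quest only to unregistered players.
; UpdateQuest advances one registered player to the next index while quests remain, and UpdateQuestForAll does so for all.
; For later indices, AddQuest calls RemoveQuest with the new index, not the previous one, before adding that quest.
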(fn `AddQuest`
  (params (`Player Controller` :type "/Game/Player/BP_PlayerController Object Reference") (`Quest index` :type Integer))
  (bind _quests (`self.Quests`))
  (bind _players (`self.Players`))
  (if (< `Quest index` (`KismetArrayLibrary.Array_Length` _quests))
    (if (== `Quest index` 0)
      (if (not (`BlueprintMapLibrary.Map_Contains` (`self.Players`) `Player Controller`))
        (`BlueprintMapLibrary.Map_Add` _players `Player Controller`)
        (`/Game/Player/BP_PlayerController.AddQuest` `Player Controller` (`|GetArrayItem` _quests `Quest index`) :!label _label))
      (else
        (`self.RemoveQuest` `Player Controller` `Quest index`)
        (`BlueprintMapLibrary.Map_Add` _players `Player Controller` `Quest index`)
        (goto _label)))))

(fn `RemoveQuest`
  (params (`Player Controller` :type "/Game/Player/BP_PlayerController Object Reference") (Index :type Integer))
  (bind _output_name (break `Quest` (`|GetArrayItem` (`self.Quests`) Index)))
  (`/Game/Player/BP_PlayerController.RemoveQuest` `Player Controller` _output_name))

(fn `UpdateQuest`
  (params (`Player Controller` :type "/Game/Player/BP_PlayerController Object Reference"))
  (bind (_value _returnvalue) (`BlueprintMapLibrary.Map_Find` (`self.Players`) `Player Controller`))
  (if _returnvalue
    (`self.AddQuest` `Player Controller` (+ _value 1))))

(fn `UpdateQuestForAll`
  (bind _keys (`BlueprintMapLibrary.Map_Keys` (`self.Players`)))
  (for _array_element _keys
    (`self.UpdateQuest` _array_element)))