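; Save game object that stores player, quest, dropped item, altar and statue state, and writes itself to its save slot.
; Each category is an array of structs with a save and a load function, looked up by linear search on Name.
; Saves replace the entry with a matching name or append one, except player data, which always appends, so loading returns the earliest match.
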(fn `LoadAltarData`
  (params (Name :type String))
  (returns (`Altar data` :type "/Game/Blueprints/Struct_AltarData Structure"))
  (for _array_element (`self.AltarData`)
    (if (`KismetStringLibrary.EqualEqual_StrStr` Name (`.Name_2_C588D0B04CC064D8A9A6C393DEDABF66` (break `/Game/Blueprints/Struct_AltarData` _array_element)))
      (return _array_element))))

(fn `LoadDropData`
  (params (Name :type String))
  (returns (DropData :type "/Game/Blueprints/Struct_DropItemData Structure"))
  (for _array_element (`self.DropData`)
    (if (`KismetStringLibrary.EqualEqual_StrStr` Name (break `/Game/Blueprints/Struct_DropItemData` _array_element))
      (return (make `/Game/Blueprints/Struct_DropItemData` (break `/Game/Blueprints/Struct_DropItemData` _array_element) (`.Deleted_5_5EE349A446AF5ABF34FEC6B4A654DDAE` (break `/Game/Blueprints/Struct_DropItemData` _array_element)))))))

(fn `LoadPlayerData`
  (params (Name :type String))
  (returns (`Player data` :type "/Game/Blueprints/Struct_PlayerData Structure"))
  (for _array_element (`self.PlayerData`)
    (if (`KismetStringLibrary.EqualEqual_StrStr` Name (`.Name_13_7742B1BF4900F0122B3B2689E0844DF4` (break `/Game/Blueprints/Struct_PlayerData` _array_element)))
      (return (make `/Game/Blueprints/Struct_PlayerData` (break `/Game/Blueprints/Struct_PlayerData` _array_element) (`.Items_7_F7ED15EB4E27F38EFCD6D994A3761333` (break `/Game/Blueprints/Struct_PlayerData` _array_element)) (`.Quests_10_576ED3334B1F33910357DF9B3F816C41` (break `/Game/Blueprints/Struct_PlayerData` _array_element)) (`.Name_13_7742B1BF4900F0122B3B2689E0844DF4` (break `/Game/Blueprints/Struct_PlayerData` _array_element)) (`.PlayerClass_16_D7F02C1148916DD0AD6532AD36784C84` (break `/Game/Blueprints/Struct_PlayerData` _array_element)))))))

(fn `LoadQuestData`
  (params (Name :type String))
  (returns (`Quest data` :type "/Game/Blueprints/Struct_QuestData Structure"))
  (for _array_element (`self.QuestData`)
    (if (`KismetStringLibrary.EqualEqual_StrStr` Name (break `/Game/Blueprints/Struct_QuestData` _array_element))
      (return (make `/Game/Blueprints/Struct_QuestData` (break `/Game/Blueprints/Struct_QuestData` _array_element) (`.Players_4_C588D0B04CC064D8A9A6C393DEDABF66` (break `/Game/Blueprints/Struct_QuestData` _array_element)))))))

(fn `LoadStatueData`
  (params (Name :type String))
  (returns (`Statue data` :type "/Game/Blueprints/Struct_StatueData Structure"))
  (for _array_element (`self.StatueData`)
    (if (`KismetStringLibrary.EqualEqual_StrStr` Name (break `/Game/Blueprints/Struct_StatueData` _array_element))
      (return (make `/Game/Blueprints/Struct_StatueData` (break `/Game/Blueprints/Struct_StatueData` _array_element) (`.State_5_5241A3404B51B3133AF0CAB92FBF38D5` (break `/Game/Blueprints/Struct_StatueData` _array_element)))))))

(fn `SaveAll`
  (`GameplayStatics.SaveGameToSlot` self (`self.Slot`)))

(fn `SaveAltarData`
  (params (Data :type "/Game/Blueprints/Struct_AltarData Structure"))
  (bind _altardata (`self.AltarData`))
  (for (_array_element _array_index) _altardata
    (if (`KismetStringLibrary.EqualEqual_StrStr` (`.Name_2_C588D0B04CC064D8A9A6C393DEDABF66` (break `/Game/Blueprints/Struct_AltarData` Data)) (break `/Game/Blueprints/Struct_AltarData` _array_element))
      (`KismetArrayLibrary.Array_Set` (`self.AltarData`) _array_index Data)
      (return)))
  (`KismetArrayLibrary.Array_Add` _altardata Data))

(fn `SaveDropData`
  (params (Data :type "/Game/Blueprints/Struct_DropItemData Structure"))
  (bind _dropdata (`self.DropData`))
  (for (_array_element _array_index) _dropdata
    (if (`KismetStringLibrary.EqualEqual_StrStr` (`.Name_2_C588D0B04CC064D8A9A6C393DEDABF66` (break `/Game/Blueprints/Struct_DropItemData` Data)) (break `/Game/Blueprints/Struct_DropItemData` _array_element))
      (`KismetArrayLibrary.Array_Set` (`self.DropData`) _array_index Data)
      (return)))
  (`KismetArrayLibrary.Array_Add` _dropdata Data))

(fn `SavePlayerData`
  (params (Data :type "/Game/Blueprints/Struct_PlayerData Structure"))
  (`KismetArrayLibrary.Array_Add` (`self.PlayerData`) Data))

(fn `SaveQuestData`
  (params (Data :type "/Game/Blueprints/Struct_QuestData Structure"))
  (bind _questdata (`self.QuestData`))
  (for (_array_element _array_index) _questdata
    (if (`KismetStringLibrary.EqualEqual_StrStr` (`.Name_8_49CFCD0848D4F1ABEBD2BCB460093BE3` (break `/Game/Blueprints/Struct_QuestData` Data)) (break `/Game/Blueprints/Struct_QuestData` _array_element))
      (`KismetArrayLibrary.Array_Set` (`self.QuestData`) _array_index Data)
      (return)))
  (`KismetArrayLibrary.Array_Add` _questdata Data))

(fn `SaveStatueData`
  (params (Data :type "/Game/Blueprints/Struct_StatueData Structure"))
  (bind _statuedata (`self.StatueData`))
  (for (_array_element _array_index) _statuedata
    (if (`KismetStringLibrary.EqualEqual_StrStr` (`.Name_2_C588D0B04CC064D8A9A6C393DEDABF66` (break `/Game/Blueprints/Struct_StatueData` Data)) (break `/Game/Blueprints/Struct_StatueData` _array_element))
      (`KismetArrayLibrary.Array_Set` (`self.StatueData`) _array_index Data)
      (return)))
  (`KismetArrayLibrary.Array_Add` _statuedata Data))