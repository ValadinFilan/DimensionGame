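; BP_GameMode is the game mode that coordinates saving and loading of game state.
; On BeginPlay it creates a fresh outgoing save object and, if the game instance's DownloadGame flag is set, async-loads the "GameSave" slot.
; Loading and SaveGame notify all BP_DataLoaderInterface actors and fire callbacks.
; Loading carries DropData into the outgoing object, which SaveGame finalizes with SaveAll; LoadGame is an empty stub.
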(event `self.ReceiveBeginPlay`
  (bind _asbp_global_game_instance (cast `/Game/Blueprints/BP_GlobalGameInstance` (`GameplayStatics.GetGameInstance`)))
  (if (`/Game/Blueprints/BP_GlobalGameInstance.DownloadGame` _asbp_global_game_instance)
    (bind _savegame (`AsyncActionHandleSaveGame.AsyncLoadGameFromSlot` "GameSave")
      (:`then`
        (bind _returnvalue (`|GenericCreateObject` "/Game/Blueprints/BP_SaveGame.BP_SaveGame_C" self :!label _label))
        (set `self.OutSavingObject` _returnvalue))
      (:`Completed`
        (bind _asbp_save_game (cast `/Game/Blueprints/BP_SaveGame` _savegame))
        (bind _output_get (set `self.SavingObject` _asbp_save_game))
        (bind _outactors (`GameplayStatics.GetAllActorsWithInterface` "/Game/Blueprints/BP_DataLoaderInterface.BP_DataLoaderInterface_C"))
        (for _array_element _outactors
          (message `/Game/Blueprints/BP_DataLoaderInterface.LoadDataFromSaveObject` _array_element))
        (`self.OnSaveLoad`)
        (set `/Game/Blueprints/BP_SaveGame.DropData` (`/Game/Blueprints/BP_SaveGame.DropData` _output_get) (`self.OutSavingObject`))))
    (else
      (goto _label))))

(fn `LoadGame`)

(fn `SaveGame`
  (bind _outactors (`GameplayStatics.GetAllActorsWithInterface` "/Game/Blueprints/BP_DataLoaderInterface.BP_DataLoaderInterface_C"))
  (for _array_element _outactors
    (message `/Game/Blueprints/BP_DataLoaderInterface.SaveDataToSaveObject` _array_element))
  (`self.OnSaveGame`)
  (`/Game/Blueprints/BP_SaveGame.SaveAll` (`self.OutSavingObject`)))

(fn `UserConstructionScript`)