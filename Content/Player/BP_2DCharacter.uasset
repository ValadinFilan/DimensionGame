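; Player character Blueprint for 2D-style movement, with jumping and interaction.
; The MoveRight axis moves along the control yaw's forward vector, while LookUp and Turn do nothing and the spring arm rotation code is disconnected.
; Jump sets a higher Z velocity when the character is moving than when still, and tracks a JumpPressed flag.
; Interact passes the PlayerGameController to a valid TargetActor, which is not assigned in these graphs.
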(event `InputAxis|MoveRight`
  (params (AxisValue :type "Float (single-precision)"))
  (`self.AddMovementInput` (* (`KismetMathLibrary.GetForwardVector` (`KismetMathLibrary.MakeRotator` 0.0 0.0 (.yaw (`self.GetControlRotation`)))) AxisValue)))

(event `InputAxis|LookUp`
  (params (AxisValue :type "Float (single-precision)")))

(event `InputAxis|Turn`
  (params (AxisValue :type "Float (single-precision)")))

(event `InputAction|Jump`
  (params (Key :type "Key Structure"))
  (bind _charactermovement (`self.CharacterMovement`))
  (:`Pressed`
    (if (> (`KismetMathLibrary.VSize` (`MovementComponent.Velocity` (`self.CharacterMovement`))) 0.0)
      (`self.Jump`)
      (set `CharacterMovementComponent.JumpZVelocity` 480.0 _charactermovement)
      (set `self.JumpPressed` true)
      (else
        (`self.Jump`)
        (set `CharacterMovementComponent.JumpZVelocity` 440.0 _charactermovement)
        (set `self.JumpPressed` true))))
  (:`Released`
    (set `self.JumpPressed` false)))

(event `InputAction|Interact`
  (params (Key :type "Key Structure"))
  (:`Pressed`
    (if (`KismetSystemLibrary.IsValid` (`self.TargetActor`))
      (bind _asplayer_game_controller (cast `PlayerGameController` (`self.GetController`)))
      (`InteractingActor.Interact` (`self.TargetActor`) _asplayer_game_controller))))

(fn `UserConstructionScript`)