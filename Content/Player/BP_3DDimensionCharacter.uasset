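; Player character for what the name suggests is a 3D dimension, handling movement, look, run, jump and interaction input.
; Movement follows control yaw only, while Run toggles walk speed between two values.
; Jump picks a higher Z velocity when the character is moving, and Run and Jump record pressed flags.
; Interact passes the PlayerGameController to a valid TargetActor, which is not assigned in these graphs.
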(event `InputAxis|MoveForward`
  (params (AxisValue :type "Float (single-precision)"))
  (`self.AddMovementInput` (`KismetMathLibrary.GetForwardVector` (`KismetMathLibrary.MakeRotator` 0.0 0.0 (.yaw (`self.GetControlRotation`)))) AxisValue))

(event `InputAxis|MoveRight`
  (params (AxisValue :type "Float (single-precision)"))
  (`self.AddMovementInput` (`KismetMathLibrary.GetRightVector` (`KismetMathLibrary.MakeRotator` 0.0 0.0 (.yaw (`self.GetControlRotation`)))) AxisValue))

(event `InputAxis|LookUp`
  (params (AxisValue :type "Float (single-precision)"))
  (`self.AddControllerPitchInput` AxisValue))

(event `InputAxis|Turn`
  (params (AxisValue :type "Float (single-precision)"))
  (`self.AddControllerYawInput` AxisValue))

(event `InputAction|Run`
  (params (Key :type "Key Structure"))
  (bind _charactermovement (`self.CharacterMovement`))
  (:`Pressed`
    (set `self.RunPressed` true)
    (set `CharacterMovementComponent.MaxWalkSpeed` 450.0 _charactermovement))
  (:`Released`
    (set `self.RunPressed` false)
    (set `CharacterMovementComponent.MaxWalkSpeed` 200.0 _charactermovement)))

(event `InputAction|Jump`
  (params (Key :type "Key Structure"))
  (bind _charactermovement (`self.CharacterMovement`))
  (:`Pressed`
    (if (> (`KismetMathLibrary.VSize` (`MovementComponent.Velocity` (`self.CharacterMovement`))) 0.0)
      (`self.Jump`)
      (set `CharacterMovementComponent.JumpZVelocity` 365.0 _charactermovement)
      (set `self.JumpPressed` true)
      (else
        (`self.Jump`)
        (set `CharacterMovementComponent.JumpZVelocity` 340.0 _charactermovement)
        (set `self.JumpPressed` true))))
  (:`Released`
    (set `self.JumpPressed` false)))

(event `InputAction|Interact`
  (params (Key :type "Key Structure"))
  (:`Pressed`
    (if (`KismetSystemLibrary.IsValid` (`self.TargetActor`))
      (bind _asplayer_game_controller (cast `PlayerGameController` (`self.GetController`)))
      (`InteractingActor.Interact` (`self.TargetActor`) _asplayer_game_controller))))

(fn `UserConstructionScript`
  (`parent.UserConstructionScript`))