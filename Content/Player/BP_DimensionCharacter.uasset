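; Player character that interacts with objects, teleports through portals and opens the game menu.
; Each tick a camera line trace finds the InteractingActor in view, shows its prompt if enabled, and the Interact input triggers it.
; An assigned Portal shows a help hint and enables teleporting via the Teleportation input.
; Prompts, hints and the menu are routed through BP_PlayerController.
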(event `self.ReceiveTick`
  (params (DeltaSeconds :type "Float (single-precision)"))
  (`self.TraceInteractingObject`))

(event `self.ReceivePossessed`
  (params (NewController :type "Controller Object Reference"))
  (if (`KismetSystemLibrary.IsValid` (`self.Portal`))
    (`self.SendHelpMessage` "Нажмите \"T\" чтобы телепортироваться")))

(event `InputAction|Teleportation`
  (params (Key :type "Key Structure"))
  (bind _portal (`self.Portal`))
  (:`Pressed`
    (if (`KismetSystemLibrary.IsValid` _portal)
      (`self.SendHelpMessage` "")
      (`/Game/WorldEntities/BP_Portal.Teleport` _portal self))))

(event `InputAction|Interact`
  (params (Key :type "Key Structure"))
  (bind _targetactor (`self.TargetActor`))
  (:`Pressed`
    (if (`KismetSystemLibrary.IsValid` _targetactor)
      (if (`ActingActor.Enabled` _targetactor)
        (bind _asplayer_game_controller (cast `PlayerGameController` (`self.GetController`)))
        (`InteractingActor.Interact` (`self.TargetActor`) _asplayer_game_controller)))))

(event `InputAction|Menu`
  (params (Key :type "Key Structure"))
  (:`Pressed`
    (bind _asbp_player_controller (cast `/Game/Player/BP_PlayerController` (`self.GetController`)))
    (`/Game/Player/BP_PlayerController.ShowMenu` _asbp_player_controller)))

(fn `DeletePortal`
  (set `self.Portal` null)
  (`self.SendHelpMessage` ""))

(fn `SendHelpMessage`
  (params (Message :type String))
  (bind _asbp_player_controller (cast `/Game/Player/BP_PlayerController` (`self.GetController`)))
  (`/Game/Player/BP_PlayerController.ShowHelpMessage` _asbp_player_controller Message))

(fn `SendInteractionMessage`
  (params (Message :type String))
  (bind _asbp_player_controller (cast `/Game/Player/BP_PlayerController` (`self.GetController`)))
  (`/Game/Player/BP_PlayerController.ShowInteractMessage` _asbp_player_controller Message))

(fn `SetPortal`
  (params (PortalObject :type "/Game/WorldEntities/BP_Portal Object Reference"))
  (set `self.Portal` PortalObject)
  (`self.SendHelpMessage` "Нажмите \"T\" чтобы телепортироваться"))

(fn `TraceInteractingObject`
  (bind _camera (`self.Camera`))
  (bind _returnvalue (`SceneComponent.K2_GetComponentLocation` _camera))
  (bind _outhit (`KismetSystemLibrary.LineTraceSingle` _returnvalue (+ _returnvalue (* (`SceneComponent.GetForwardVector` _camera) (`self.View distatce`))) "TraceTypeQuery1"))
  (bind _asinteracting_actor (cast `InteractingActor` (`.HitActor` (`GameplayStatics.BreakHitResult` _outhit)))
    (:`then`
      (bind _output_get (set `self.TargetActor` _asinteracting_actor))
      (if (`ActingActor.Enabled` _output_get)
        (`self.SendInteractionMessage` (`KismetStringLibrary.Concat_StrStr` "\"Е\" " (`InteractingActor.InteractingText` _output_get)))))
    (:`CastFailed`
      (set `self.TargetActor` null)
      (`self.SendInteractionMessage` ""))))

(fn `UserConstructionScript`)