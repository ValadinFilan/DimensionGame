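; Player controller that owns the player's inventory and quest list and handles the win event, menu and save/load.
; Inventory and quest changes, messages, menu toggles and the delayed win screen reach the UI by casting the HUD to BP_GameInterface.
; Saving records pawn transform, class, items and quests.
; When DownloadGame is set, loading restores them by spawning and possessing the saved class, raised in Z unless 3D, then destroying the old pawn.
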(event `self.ReceiveBeginPlay`
  (add `self.WinEvent` (delegate `WinEvent_Event`))
  (`KismetSystemLibrary.Delay` 0.1)
  (`self.UpdateQuests`)
  (`self.UpdateInventory`))

(event `WinEvent_Event`
  (`KismetSystemLibrary.Delay` 3.0)
  (bind _asbp_game_interface (cast `/Game/UI/BP_GameInterface` (`self.GetHUD`)))
  (`/Game/UI/BP_GameInterface.ShowWin` _asbp_game_interface))

(event `/Game/Blueprints/BP_DataLoaderInterface.LoadDataFromSaveObject`
  (`self.LoadDataImplementation`))

(event `/Game/Blueprints/BP_DataLoaderInterface.SaveDataToSaveObject`
  (`self.SaveData`))

(fn `AddItem`
  (params (Item :type "Item Structure"))
  (`InventoryComponent.AddItem` (`self.Inventory`) Item)
  (`self.UpdateInventory`))

(fn `AddQuest`
  (params (Quest :type "Quest Structure"))
  (`KismetArrayLibrary.Array_Add` (`self.Quests`) Quest)
  (`self.UpdateQuests`))

(fn `CloseMenu`
  (bind _asbp_game_interface (cast `/Game/UI/BP_GameInterface` (`self.GetHUD`)))
  (`/Game/UI/BP_GameInterface.CloseMenu` _asbp_game_interface))

(fn `HasItem`
  (params (ItemName :type String))
  (returns (Rusult :type Boolean))
  (bind _returnvalue (`InventoryComponent.IsItemInInventory` (`self.Inventory`) ItemName))
  (return _returnvalue))

(fn `LoadDataImplementation`
  (bind _asbp_global_game_instance (cast `/Game/Blueprints/BP_GlobalGameInstance` (`GameplayStatics.GetGameInstance`)))
  (if (`/Game/Blueprints/BP_GlobalGameInstance.DownloadGame` _asbp_global_game_instance)
    (bind _player_data (`/Game/Blueprints/BP_SavingLib.LoadPlayerData` self))
    (set `InventoryComponent.Items` (`.Items_7_F7ED15EB4E27F38EFCD6D994A3761333` (break `/Game/Blueprints/Struct_PlayerData` _player_data)) (`self.Inventory`))
    (set `self.Quests` (`.Quests_10_576ED3334B1F33910357DF9B3F816C41` (break `/Game/Blueprints/Struct_PlayerData` _player_data)))
    (set `self.LastPlayer` (`self.K2_GetPawn`))
    (if (== (`.PlayerClass_16_D7F02C1148916DD0AD6532AD36784C84` (break `/Game/Blueprints/Struct_PlayerData` _player_data)) "/Game/Player/BP_3DDimensionCharacter.BP_3DDimensionCharacter_C")
      (bind _returnvalue (`|SpawnActorFromClass` (`.PlayerClass_16_D7F02C1148916DD0AD6532AD36784C84` (break `/Game/Blueprints/Struct_PlayerData` _player_data)) (break `/Game/Blueprints/Struct_PlayerData` _player_data) "AdjustIfPossibleButAlwaysSpawn" "OverrideRootScale" null null))
      (`self.Possess` _returnvalue)
      (else
        (bind _scale (.scale (break `/Game/Blueprints/Struct_PlayerData` _player_data)))
        (bind _returnvalue_2 (`|SpawnActorFromClass` (`.PlayerClass_16_D7F02C1148916DD0AD6532AD36784C84` (break `/Game/Blueprints/Struct_PlayerData` _player_data)) (`KismetMathLibrary.MakeTransform` (`KismetMathLibrary.MakeVector` (.x (.location (break `/Game/Blueprints/Struct_PlayerData` _player_data))) (.y (.location (break `/Game/Blueprints/Struct_PlayerData` _player_data))) (+ (.z (.location (break `/Game/Blueprints/Struct_PlayerData` _player_data))) 500.0)) (.rotation (break `/Game/Blueprints/Struct_PlayerData` _player_data)) _scale) "AdjustIfPossibleButAlwaysSpawn" "OverrideRootScale" null null))
        (`self.SetActorScale3D` _returnvalue_2 _scale)
        (`self.Possess` _returnvalue_2)))
    (`self.K2_DestroyActor` (`self.LastPlayer`))))

(fn `RemoveItem`
  (params (`Item name` :type String))
  (returns (Item :type "Item Structure"))
  (bind _returnvalue (`InventoryComponent.GetItem` (`self.Inventory`) `Item name`))
  (`self.UpdateInventory`)
  (return _returnvalue))

(fn `RemoveQuest`
  (params (QuestName :type String))
  (for (_array_element _array_index) (`self.Quests`)
    (if (`KismetStringLibrary.EqualEqual_StrStr` (break `Quest` _array_element) QuestName)
      (`KismetArrayLibrary.Array_Remove` (`self.Quests`) _array_index)
      (`self.UpdateQuests`))))

(fn `SaveData`
  (bind _returnvalue (`self.K2_GetPawn`))
  (bind _asdimention_character (cast `DimentionCharacter` _returnvalue))
  (`/Game/Blueprints/BP_SavingLib.SavePlayerData` (make `/Game/Blueprints/Struct_PlayerData` (`self.GetTransform` _returnvalue) (`InventoryComponent.Items` (`self.Inventory`)) (`self.Quests`) (`KismetSystemLibrary.GetObjectName` self) (`GameplayStatics.GetObjectClass` _asdimention_character)) self))

(fn `ShowHelpMessage`
  (params (Message :type String))
  (bind _asbp_game_interface (cast `/Game/UI/BP_GameInterface` (`self.GetHUD`)))
  (`/Game/UI/BP_GameInterface.ShowHelpMessage` _asbp_game_interface Message))

(fn `ShowInteractMessage`
  (params (Message :type String))
  (bind _returnvalue (`self.GetHUD`))
  (if (`KismetSystemLibrary.IsValid` _returnvalue)
    (bind _asbp_game_interface (cast `/Game/UI/BP_GameInterface` _returnvalue))
    (`/Game/UI/BP_GameInterface.ShowMessage` _asbp_game_interface Message)))

(fn `ShowMenu`
  (bind _asbp_game_interface (cast `/Game/UI/BP_GameInterface` (`self.GetHUD`)))
  (`/Game/UI/BP_GameInterface.ShowMenu` _asbp_game_interface))

(fn `UpdateInventory`
  (bind _asbp_game_interface (cast `/Game/UI/BP_GameInterface` (`self.GetHUD`)))
  (`/Game/UI/BP_GameInterface.UpdateInventory` _asbp_game_interface (`InventoryComponent.Items` (`self.Inventory`))))

(fn `UpdateQuest`
  (params (`Last quest` :type "Quest Structure") (`New quest` :type "Quest Structure"))
  (bind _quests (`self.Quests`))
  (for (_array_element _array_index) _quests
    (if (`KismetStringLibrary.EqualEqual_StrStr` (break `Quest` _array_element) `Last quest_Name`)
      (`KismetArrayLibrary.Array_Set` _quests _array_index `New quest`)
      (`self.UpdateQuests` :!label _label)
      (return)))
  (`self.AddQuest` `New quest`)
  (goto _label))

(fn `UpdateQuests`
  (bind _asbp_game_interface (cast `/Game/UI/BP_GameInterface` (`self.GetHUD`)))
  (`/Game/UI/BP_GameInterface.UpdateQuests` _asbp_game_interface (`self.Quests`)))

(fn `UserConstructionScript`)

(fn `Win`
  (`self.WinEvent`))