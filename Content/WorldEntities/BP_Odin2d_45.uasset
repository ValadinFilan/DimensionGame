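; Rotatable 2D Odin statue, apparently a puzzle piece, that cycles through numbered facing states when interacted with.
; Each turn hides the sprite behind a temporary flipbook for a second, then shows that state's sprite.
; Reaching TargetState sets IsMetCondition and notifies the Manager.
; The construction script previews the starting state and pre-checks the target; State is saved and restored, with loading replaying the turn animation.
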(event `Confirm Rotation`
  (bind _returnvalue (`KismetMathLibrary.MakeTransform` (0.0 0.0 0.0)))
  ;[1 1 1] Animation
  (`SceneComponent.SetVisibility` (`self.PaperSprite`) false false)
  (switch `int` (`self.State`)
    (:`1`
      (bind _returnvalue_2 (`AddComponent|NODE_AddPaperFlipbookComponent-16` :`RelativeTransform` _returnvalue))
      (`KismetSystemLibrary.Delay` 1.0)
      (`PaperSpriteComponent.SetSprite` (`self.PaperSprite`) "/Game/Sprites/Odin/odinBGO_tex_Sprite_29.odinBGO_tex_Sprite_29")
      (`ActorComponent.K2_DestroyComponent` _returnvalue_2))
    (:`2`
      (bind _returnvalue_3 (`AddComponent|NODE_AddPaperFlipbookComponent-17` :`RelativeTransform` _returnvalue))
      (`KismetSystemLibrary.Delay` 1.0)
      (`PaperSpriteComponent.SetSprite` (`self.PaperSprite`) "/Game/Sprites/Odin/odinBGO_tex_Sprite_45.odinBGO_tex_Sprite_45")
      (`ActorComponent.K2_DestroyComponent` _returnvalue_3))
    (:`3`
      (bind _returnvalue_4 (`AddComponent|NODE_AddPaperFlipbookComponent-18` :`RelativeTransform` _returnvalue))
      (`KismetSystemLibrary.Delay` 1.0)
      (`PaperSpriteComponent.SetSprite` (`self.PaperSprite`) "/Game/Sprites/Odin/odinBGO_tex_Sprite_61.odinBGO_tex_Sprite_61")
      (`ActorComponent.K2_DestroyComponent` _returnvalue_4))
    (:`4`
      (bind _returnvalue_5 (`AddComponent|NODE_AddPaperFlipbookComponent-19` :`RelativeTransform` _returnvalue))
      (`KismetSystemLibrary.Delay` 1.0)
      (`PaperSpriteComponent.SetSprite` (`self.PaperSprite`) "/Game/Sprites/Odin/odinBGO_tex_Sprite_13.odinBGO_tex_Sprite_13")
      (`ActorComponent.K2_DestroyComponent` _returnvalue_5)))
  (`SceneComponent.SetVisibility` (`self.PaperSprite`) true false))

(event `self.ReceiveBeginPlay`
  (add `InteractingActor.OnInteract` (delegate `OnInteract_Event_1`)))

(event `OnInteract_Event_1`
  (params (PlayerController :type "PlayerGameController Object Reference"))
  (if (`self.Enabled`)
    (`self.ChangeState`)
    (`self.Confirm Rotation`)
    ;[1 1 1] Interaction
    (set `self.isRotating` false)
    (if (== (`self.State`) (`self.TargetState`))
      (set `self.Enabled` true)
      (set `self.IsMetCondition` true)
      (if (`KismetSystemLibrary.IsValid` (`self.Manager`))
        (`ActorManager.UpdateManager` (`self.Manager`) self)))))

(event `/Game/Blueprints/BP_DataLoaderInterface.LoadDataFromSaveObject`
  (bind _drop_data (`/Game/Blueprints/BP_SavingLib.LoadStatueData` self))
  (set `self.State` (`.State_5_5241A3404B51B3133AF0CAB92FBF38D5` (break `/Game/Blueprints/Struct_StatueData` _drop_data)))
  (`self.Confirm Rotation`))

(event `/Game/Blueprints/BP_DataLoaderInterface.SaveDataToSaveObject`
  (`/Game/Blueprints/BP_SavingLib.SaveStatueData` (make `/Game/Blueprints/Struct_StatueData` (`KismetSystemLibrary.GetObjectName` self) (`self.State`)) self))

(fn `ChangeState`
  (if (not (`self.isRotating`))
    (set `self.State` (+ (mod (`self.State`) (`self.Number of states`)) 1))
    (set `self.Rotated` 0.0)
    (set `self.isRotating` true)))

(fn `UserConstructionScript`
  (switch `int` (`self.State`)
    (:`1`
      (`PaperSpriteComponent.SetSprite` (`self.PaperSprite`) "/Game/Sprites/Odin/odinBGO_tex_Sprite_29.odinBGO_tex_Sprite_29"))
    (:`2`
      (`PaperSpriteComponent.SetSprite` (`self.PaperSprite`) "/Game/Sprites/Odin/odinBGO_tex_Sprite_45.odinBGO_tex_Sprite_45"))
    (:`3`
      (`PaperSpriteComponent.SetSprite` (`self.PaperSprite`) "/Game/Sprites/Odin/odinBGO_tex_Sprite_61.odinBGO_tex_Sprite_61"))
    (:`4`
      (`PaperSpriteComponent.SetSprite` (`self.PaperSprite`) "/Game/Sprites/Odin/odinBGO_tex_Sprite_13.odinBGO_tex_Sprite_13")))
  (if (== (`self.State`) (`self.TargetState`))
    (set `self.IsMetCondition` true)))