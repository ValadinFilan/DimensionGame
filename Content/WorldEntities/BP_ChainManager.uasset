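; Puzzle manager for a chain of altars that must be triggered in order, rewarding completion with a rune.
; Each OnUpdateManager call disables the sender and sets its Condition flag only if all earlier ones are set, otherwise deactivating every altar.
; When all flags are set, it spawns BP_Rune1, calls Act on its Targets and updates the quest.
; A sphere overlap gives the entering player that quest.
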(event `self.ReceiveBeginPlay`
  (add `self.OnUpdateManager` (delegate `OnUpdateManager_Event_1`)))

(event `OnUpdateManager_Event_1` :!signature `self.OnUpdateManager`
  (params (Actor :type "InteractingActor Object Reference"))
  (set `ActingActor.Enabled` false Actor)
  (bind _success (`self.SetBools` Actor))
  (if _success
    (`self.CheckAll`)
    (else
      (for _array_element (`self.Actors`)
        (bind _asbp_activate_chain_altar (cast `/Game/WorldEntities/BP_ActivateChainAltar` _array_element))
        (set `/Game/WorldEntities/BP_ActivateChainAltar.Active` false _asbp_activate_chain_altar)))))

(event `self.Sphere.OnComponentBeginOverlap`
  (params (OverlappedComponent :type "PrimitiveComponent Object Reference") (OtherActor :type "Actor Object Reference") (OtherComp :type "PrimitiveComponent Object Reference") (OtherBodyIndex :type Integer) (bFromSweep :type Boolean) (SweepResult :type "HitResult Structure (by ref)"))
  (bind _asbp_dimension_character (cast `/Game/Player/BP_DimensionCharacter` OtherActor))
  (bind _asbp_player_controller (cast `/Game/Player/BP_PlayerController` (`Pawn.GetController` _asbp_dimension_character)))
  (`/Game/Blueprints/BP_QuestComponent.AddQuest` (`self.BP_QuestComponent`) _asbp_player_controller 0))

(fn `CheckAll`
  (for _array_element (`self.Condition`)
    (if (not _array_element)
      (return)))
  (`|SpawnActorFromClass` "/Game/WorldEntities/BP_Rune1.BP_Rune1_C" (`self.GetTransform`) "Undefined" "OverrideRootScale" null null)
  (for _array_element_2 (`self.Targets`)
    (`ActingActor.Act` _array_element_2)
    (`/Game/Blueprints/BP_QuestComponent.UpdateQuestForAll` (`self.BP_QuestComponent`))))

(fn `SetBools`
  (params (Actor :type "InteractingActor Object Reference"))
  (returns (Success :type Boolean))
  (bind _condition (`self.Condition`))
  (for (_array_element _array_index) (`self.Actors`)
    (if (== _array_element Actor)
      (`KismetArrayLibrary.Array_Set` _condition _array_index true)
      (return true)
      (elif (not (`|GetArrayItem` _condition _array_index))
        (return false)))))

(fn `UserConstructionScript`
  (for _ (`self.Actors`)
    (`KismetArrayLibrary.Array_Add` (`self.Condition`))))