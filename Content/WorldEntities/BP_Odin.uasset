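; BP_Odin is an interactable rotating statue puzzle piece that must be turned to a target state.
; Each interaction cycles State and starts a yaw turn of one even step of a full circle, animated on Tick.
; Finishing on TargetState disables the statue, marks its condition met and notifies its Manager.
; State is saved and loaded, with rotation and condition rebuilt from it on load and construction.
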(event `self.ReceiveBeginPlay`
  (add `InteractingActor.OnInteract` (delegate `OnInteract_Event_0`)))

(event `OnInteract_Event_0`
  (params (PlayerController :type "PlayerGameController Object Reference"))
  (`self.ChangeState`))

(event `self.ReceiveTick`
  (params (DeltaSeconds :type "Float (single-precision)"))
  (if (`self.Enabled`)
    (`self.Rotate` (* DeltaSeconds (`self.RotateVelocity`)))))

(event `/Game/Blueprints/BP_DataLoaderInterface.SaveDataToSaveObject`
  (`/Game/Blueprints/BP_SavingLib.SaveStatueData` (make `/Game/Blueprints/Struct_StatueData` (`KismetSystemLibrary.GetObjectName` self) (`self.State`)) self))

(event `/Game/Blueprints/BP_DataLoaderInterface.LoadDataFromSaveObject`
  (bind _drop_data (`/Game/Blueprints/BP_SavingLib.LoadStatueData` self))
  (set `self.State` (`.State_5_5241A3404B51B3133AF0CAB92FBF38D5` (break `/Game/Blueprints/Struct_StatueData` _drop_data)))
  (`self.ConfirmRotation`))

(fn `ChangeState`
  (if (not (`self.isRotating`))
    (set `self.State` (+ (mod (`self.State`) (`self.Number of states`)) 1))
    (set `self.Rotated` 0.0)
    (set `self.isRotating` true)))

(fn `ConfirmRotation`
  (`self.K2_SetActorRotation` (`KismetMathLibrary.MakeRotator` 0.0 0.0 (+ (* (`KismetMathLibrary.Conv_IntToDouble` (`self.State`)) (/ 360.0 (`KismetMathLibrary.Conv_IntToDouble` (`self.Number of states`)))) (`self.StartRotation`) -180.0)))
  (if (== (`self.State`) (`self.TargetState`))
    (set `self.IsMetCondition` true)
    (else
      (set `self.IsMetCondition` false))))

(fn `Rotate`
  (params (RotationVelocity :type "Float (double-precision)"))
  (if (< (`self.Rotated`) (/ 360.0 (`KismetMathLibrary.Conv_IntToDouble` (`self.Number of states`))))
    (`self.K2_AddActorLocalRotation` (`KismetMathLibrary.MakeRotator` 0.0 0.0 RotationVelocity))
    (set `self.Rotated` (+ RotationVelocity (`self.Rotated`)))
    (else
      (set `self.isRotating` false)
      (if (== (`self.State`) (`self.TargetState`))
        (set `self.Enabled` false)
        (set `self.IsMetCondition` true)
        (if (`KismetSystemLibrary.IsValid` (`self.Manager`))
          (`ActorManager.UpdateManager` (`self.Manager`) self))))))

(fn `UserConstructionScript`
  (`self.ConfirmRotation`))