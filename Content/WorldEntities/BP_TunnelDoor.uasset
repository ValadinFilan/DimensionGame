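; BP_TunnelDoor is an interactable door that consumes a required item from the player, removes a quest, then saves itself as opened and destroys itself.
; Its Act event marks it enabled and endlessly spawns lightning effects at its box on a short delay loop.
; Save and load reuse altar data, with Active meaning opened: loading either destroys the door again or restores Enabled, calling Act to restart the effect.
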(event `OnInteract_Event_0` :!signature `self.OnInteract`
  (params (PlayerController :type "PlayerGameController Object Reference"))
  (bind _requireditem (`self.RequiredItem`))
  (bind _asbp_player_controller (cast `/Game/Player/BP_PlayerController` PlayerController))
  (bind _rusult (`/Game/Player/BP_PlayerController.HasItem` _asbp_player_controller _requireditem))
  (if _rusult
    (`/Game/Player/BP_PlayerController.RemoveItem` _asbp_player_controller _requireditem)
    (`/Game/Blueprints/BP_QuestComponent.RemoveQuest` (`self.BP_QuestComponent`) _asbp_player_controller 0)
    (`KismetSystemLibrary.Delay` 1.0)
    (`/Game/Blueprints/BP_SavingLib.SaveAltarData` (make `/Game/Blueprints/Struct_AltarData` (`KismetSystemLibrary.GetObjectName` self) true (`self.Enabled`)) self)
    (`self.K2_DestroyActor`)))

(event `self.ReceiveBeginPlay`
  (add `self.OnInteract` (delegate `OnInteract_Event_0`))
  (add `self.OnAct` (delegate `OnAct_Event_0`)))

(event `OnAct_Event_0`
  (set `self.Enabled` true)
  (`NiagaraFunctionLibrary.SpawnSystemAtLocation` "/Game/Niagara/Ligthning_effect.Ligthning_effect" (`SceneComponent.K2_GetComponentLocation` (`self.Box`)) :!label _label)
  (`KismetSystemLibrary.Delay` 0.1)
  (goto _label))

(event `/Game/Blueprints/BP_DataLoaderInterface.SaveDataToSaveObject`
  (`/Game/Blueprints/BP_SavingLib.SaveAltarData` (make `/Game/Blueprints/Struct_AltarData` (`KismetSystemLibrary.GetObjectName` self) false (`self.Enabled`)) self))

(event `/Game/Blueprints/BP_DataLoaderInterface.LoadDataFromSaveObject`
  (bind _drop_data (`/Game/Blueprints/BP_SavingLib.LoadAltarData` self))
  (if (`.Active_5_B1BA00A24983A9F692D2C395674004CD` (break `/Game/Blueprints/Struct_AltarData` _drop_data))
    (`/Game/Blueprints/BP_SavingLib.SaveAltarData` (make `/Game/Blueprints/Struct_AltarData` (`KismetSystemLibrary.GetObjectName` self) (`.Active_5_B1BA00A24983A9F692D2C395674004CD` (break `/Game/Blueprints/Struct_AltarData` _drop_data)) (`.Enabled_6_78BB5ED14770876B1373DB881DA191D8` (break `/Game/Blueprints/Struct_AltarData` _drop_data))) self)
    (`self.K2_DestroyActor`)
    (else
      (bind _output_get (set `self.Enabled` (`.Enabled_6_78BB5ED14770876B1373DB881DA191D8` (break `/Game/Blueprints/Struct_AltarData` _drop_data))))
      (if _output_get
        (`self.Act`)))))

(fn `UserConstructionScript`)