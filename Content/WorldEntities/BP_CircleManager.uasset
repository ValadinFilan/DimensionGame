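; BP_CircleManager is a world entity that triggers a set of target objects once every actor in its watched group meets its condition.
; On BeginPlay it binds to the OnUpdateManager dispatcher, so checks are event-driven rather than ticked.
; Each broadcast ANDs IsMetCondition across Actors and, if all pass, calls Act on every entry in Targets.
; It keeps no fired state, so Targets act again on every passing update.
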(event `self.ReceiveBeginPlay`
  (add `self.OnUpdateManager` (delegate `OnUpdateManager_Event_1`)))

(event `OnUpdateManager_Event_1` :!signature `self.OnUpdateManager`
  (params (Actor :type "InteractingActor Object Reference"))
  (set `self.Condition` true)
  (for _array_element (`self.Actors`)
    (set `self.Condition` (and (`self.Condition`) (`ManagedInteractingActor.IsMetCondition` _array_element))))
  (if (`self.Condition`)
    (for _array_element_2 (`self.Targets`)
      (`ActingActor.Act` _array_element_2))))

(fn `UserConstructionScript`)