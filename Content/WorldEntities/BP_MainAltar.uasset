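; The main altar is an interactable quest objective that wins the game when activated with a required item.
; An Act event enables it; Interact consumes the item, even while disabled, and if enabled lights the altar, updates the quest and calls Win on player 0.
; While active, Tick eases the topstone and crystal upward and spins and bobs the crystal.
; Sphere overlap grants a state-dependent quest, and Active/Enabled persist through save data.
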(event `self.ReceiveBeginPlay`
  (add `self.OnInteract` (delegate `OnInteract_Event_0`))
  (add `self.OnAct` (delegate `OnAct_Event_0`)))

(event `OnAct_Event_0`
  (set `self.Enabled` true)
  (`/Game/Blueprints/BP_QuestComponent.UpdateQuestForAll` (`self.QuestComponent`)))

(event `OnInteract_Event_0` :!signature `self.OnInteract`
  (params (PlayerController :type "PlayerGameController Object Reference"))
  (bind _requireditem (`self.RequiredItem`))
  (bind _asbp_player_controller (cast `/Game/Player/BP_PlayerController` PlayerController))
  (bind _rusult (`/Game/Player/BP_PlayerController.HasItem` _asbp_player_controller _requireditem))
  (if _rusult
    (`/Game/Player/BP_PlayerController.RemoveItem` _asbp_player_controller _requireditem)
    (if (`self.Enabled`)
      (set `self.Active` true)
      (set `self.Enabled` false)
      (`SceneComponent.SetVisibility` (`self.PointLight`) true false)
      (`/Game/Blueprints/BP_QuestComponent.UpdateQuest` (`self.QuestComponent`) _asbp_player_controller)
      (bind _asbp_player_controller_2 (cast `/Game/Player/BP_PlayerController` (`GameplayStatics.GetPlayerController` 0)))
      (`/Game/Player/BP_PlayerController.Win` _asbp_player_controller_2))))

(event `self.ReceiveTick`
  (params (DeltaSeconds :type "Float (single-precision)"))
  (if (`self.Active`)
    (`self.SlowUp` 20.0 2.5 (* DeltaSeconds 15.0))
    (`self.MoveCristall` (* DeltaSeconds 5.0))))

(event `self.Sphere.OnComponentBeginOverlap`
  (params (OverlappedComponent :type "PrimitiveComponent Object Reference") (OtherActor :type "Actor Object Reference") (OtherComp :type "PrimitiveComponent Object Reference") (OtherBodyIndex :type Integer) (bFromSweep :type Boolean) (SweepResult :type "HitResult Structure (by ref)"))
  (bind _questcomponent (`self.QuestComponent`))
  (bind _asdimention_character (cast `DimentionCharacter` OtherActor))
  (bind _asbp_player_controller (cast `/Game/Player/BP_PlayerController` (`Pawn.GetController` _asdimention_character)))
  (if (`self.Enabled`)
    (`/Game/Blueprints/BP_QuestComponent.AddQuest` _questcomponent _asbp_player_controller 1)
    (else
      (`/Game/Blueprints/BP_QuestComponent.AddQuest` _questcomponent _asbp_player_controller 0))))

(event `/Game/Blueprints/BP_DataLoaderInterface.LoadDataFromSaveObject`
  (bind _drop_data (`/Game/Blueprints/BP_SavingLib.LoadAltarData` self))
  (set `self.Active` (`.Active_5_B1BA00A24983A9F692D2C395674004CD` (break `/Game/Blueprints/Struct_AltarData` _drop_data)))
  (set `self.Enabled` (`.Enabled_6_78BB5ED14770876B1373DB881DA191D8` (break `/Game/Blueprints/Struct_AltarData` _drop_data))))

(event `/Game/Blueprints/BP_DataLoaderInterface.SaveDataToSaveObject`
  (`/Game/Blueprints/BP_SavingLib.SaveAltarData` (make `/Game/Blueprints/Struct_AltarData` (`KismetSystemLibrary.GetObjectName` self) (`self.Active`) (`self.Enabled`)) self))

(fn `MoveCristall`
  (params (Velocity :type "Float (double-precision)"))
  (`SceneComponent.K2_AddLocalOffset` (`self.Cristall`) (`KismetMathLibrary.MakeVector` 0.0 0.0 (* Velocity (`KismetMathLibrary.Sin` (`self.SinTemp`)))) false false)
  (`SceneComponent.K2_AddLocalRotation` (`self.Cristall`) (`KismetMathLibrary.MakeRotator` 0.0 0.0 (* Velocity 4.0)) false false)
  (set `self.SinTemp` (mod (+ (`self.SinTemp`) 0.01) (* (`KismetMathLibrary.GetPI`) 2.0))))

(fn `SlowUp`
  (params (TopstoneUpBorder :type "Float (double-precision)") (CristalUpBorder :type "Float (double-precision)") (Velocity :type "Float (double-precision)"))
  (bind (_relativelocation_x _relativelocation_y _relativelocation_z) (`KismetMathLibrary.BreakVector` (`SceneComponent.RelativeLocation` (`self.Cristall`))))
  (bind (_relativelocation_x_2 _relativelocation_y_2 _relativelocation_z_2) (`KismetMathLibrary.BreakVector` (`SceneComponent.RelativeLocation` (`self.Topstone`))))
  (if (< _relativelocation_z_2 TopstoneUpBorder)
    (`SceneComponent.K2_AddLocalOffset` (`self.Topstone`) (`KismetMathLibrary.MakeVector` 0.0 0.0 (* Velocity (- 1.0 (/ (- _relativelocation_z_2 TopstoneUpBorder) 50.0)))) false false))
  (if (< _relativelocation_z CristalUpBorder)
    (`SceneComponent.K2_AddLocalOffset` (`self.Cristall`) (`KismetMathLibrary.MakeVector` 0.0 0.0 (* Velocity (- 1.0 (/ (- _relativelocation_z CristalUpBorder) 50.0)))) false false)))

(fn `UserConstructionScript`)