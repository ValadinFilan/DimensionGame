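; BP_Odin2d is an interactable 2D Odin puzzle piece that steps through rotation states toward a target.
; Each interaction advances State cyclically, hides the sprite, plays a temporary flipbook component for a second, then shows that state's sprite.
; Reaching TargetState disables the piece, marks its condition met and notifies its Manager.
; The construction script derives the actor's initial yaw from State, NumberOfStates and StartRotation.
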(event `self.ReceiveBeginPlay`
  (add `InteractingActor.OnInteract` (delegate `OnInteract_Event_1`)))

(event `OnInteract_Event_1`
  (params (PlayerController :type "PlayerGameController Object Reference"))
  (bind _returnvalue (`KismetMathLibrary.MakeTransform` (0.0 0.0 0.0)))
  (if (`self.Enabled`)
    ;[1 1 1] Animation
    (`self.ChangeState`)
    (`SceneComponent.SetVisibility` (`self.PaperSprite`) false false)
    (switch `int` (`self.State`)
      (:`1`
        (bind _returnvalue_2 (`AddComponent|NODE_AddPaperFlipbookComponent-0` :`RelativeTransform` _returnvalue))
        (`KismetSystemLibrary.Delay` 1.0)
        (`PaperSpriteComponent.SetSprite` (`self.PaperSprite`) "/Game/Sprites/Odin/odinBGO_tex_Sprite_15.odinBGO_tex_Sprite_15")
        (`ActorComponent.K2_DestroyComponent` _returnvalue_2))
      (:`2`
        (bind _returnvalue_3 (`AddComponent|NODE_AddPaperFlipbookComponent-1` :`RelativeTransform` _returnvalue))
        (`KismetSystemLibrary.Delay` 1.0)
        (`PaperSpriteComponent.SetSprite` (`self.PaperSprite`) "/Game/Sprites/Odin/odinBGO_tex_Sprite_30.odinBGO_tex_Sprite_30")
        (`ActorComponent.K2_DestroyComponent` _returnvalue_3))
      (:`3`
        (bind _returnvalue_4 (`AddComponent|NODE_AddPaperFlipbookComponent-2` :`RelativeTransform` _returnvalue))
        (`KismetSystemLibrary.Delay` 1.0)
        (`PaperSpriteComponent.SetSprite` (`self.PaperSprite`) "/Game/Sprites/Odin/odinBGO_tex_Sprite_47.odinBGO_tex_Sprite_47")
        (`ActorComponent.K2_DestroyComponent` _returnvalue_4))
      (:`4`
        (bind _returnvalue_5 (`AddComponent|NODE_AddPaperFlipbookComponent-3` :`RelativeTransform` _returnvalue))
        (`KismetSystemLibrary.Delay` 1.0)
        (`PaperSpriteComponent.SetSprite` (`self.PaperSprite`) "/Game/Sprites/Odin/odinBGO_tex_Sprite_63.odinBGO_tex_Sprite_63")
        (`ActorComponent.K2_DestroyComponent` _returnvalue_5)))
    (`SceneComponent.SetVisibility` (`self.PaperSprite`) true false)
    ;[1 1 1] Interaction
    (set `self.isRotating` false)
    (if (== (`self.State`) (`self.TargetState`))
      (set `self.Enabled` false)
      (set `self.IsMetCondition` true)
      (if (`KismetSystemLibrary.IsValid` (`self.Manager`))
        (`ActorManager.UpdateManager` (`self.Manager`))))))

(fn `ChangeState`
  (if (not (`self.isRotating`))
    (set `self.State` (+ (mod (`self.State`) (`self.Number of states`)) 1))
    (set `self.Rotated` 0.0)
    (set `self.isRotating` true)))

(fn `UserConstructionScript`
  (`self.K2_SetActorRotation` (`KismetMathLibrary.MakeRotator` 0.0 0.0 (+ (* (`KismetMathLibrary.Conv_IntToDouble` (`self.State`)) (/ 360.0 (`KismetMathLibrary.Conv_IntToDouble` (`self.Number of states`)))) (`self.StartRotation`) -180.0))))