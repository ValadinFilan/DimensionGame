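; Test interactable 3D rotating column that turns around its yaw axis in discrete, evenly spaced steps.
; The OnInteract event advances State cyclically through NumberOfStates and prints the new value.
; Tick adds local yaw at RotateVelocity only while the actor's yaw is below the target derived from State and StartZRotation.
; The construction script snaps the actor to that same angle.
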(event `self.ReceiveBeginPlay`
  (add `self.OnInteract` (delegate `OnInteract_Event_0`)))

(event `OnInteract_Event_0` :!signature `self.OnInteract`
  (params (PlayerController :type "PlayerGameController Object Reference"))
  (`self.ChangeState`))

(event `self.ReceiveTick`
  (params (DeltaSeconds :type "Float (single-precision)"))
  (`self.Rotate` (* DeltaSeconds (`self.RotateVelocity`))))

(fn `ChangeState`
  (bind _output_get (set `self.State` (+ (mod (`self.State`) (`self.Number of states`)) 1)))
  (`KismetSystemLibrary.PrintString` (`KismetStringLibrary.Conv_IntToString` _output_get)))

(fn `Rotate`
  (params (RotationVelocity :type "Float (double-precision)"))
  (bind (_returnvalue_roll _returnvalue_pitch _returnvalue_yaw) (`KismetMathLibrary.BreakRotator` (`self.K2_GetActorRotation`)))
  (if (< _returnvalue_yaw (+ (* (`KismetMathLibrary.Conv_IntToDouble` (`self.State`)) (/ 360.0 (`KismetMathLibrary.Conv_IntToDouble` (`self.Number of states`)))) (`self.StartZRotation`) -180.0))
    (`self.K2_AddActorLocalRotation` (`KismetMathLibrary.MakeRotator` 0.0 0.0 RotationVelocity))))

(fn `UserConstructionScript`
  (`self.K2_SetActorRotation` (`KismetMathLibrary.MakeRotator` 0.0 0.0 (+ (* (`KismetMathLibrary.Conv_IntToDouble` (`self.State`)) (/ 360.0 (`KismetMathLibrary.Conv_IntToDouble` (`self.Number of states`)))) (`self.StartZRotation`) -180.0))))