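; Test playable 2D character that takes over from a DimentionCharacter when that character enters its Sphere.
; The overlap blends the PlayerGameController's view to this actor over two seconds, then possesses it and destroys the old character.
; Movement uses only the MoveRight axis along control-yaw forward, with empty look and turn handlers.
; Jump velocity is higher when already moving, and Interact forwards the controller to a valid TargetActor.
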(event `self.Sphere.OnComponentBeginOverlap`
  (params (OverlappedComponent :type "PrimitiveComponent Object Reference") (OtherActor :type "Actor Object Reference") (OtherComp :type "PrimitiveComponent Object Reference") (OtherBodyIndex :type Integer) (bFromSweep :type Boolean) (SweepResult :type "HitResult Structure (by ref)"))
  (bind _asdimention_character (cast `DimentionCharacter` OtherActor))
  (bind _asplayer_game_controller (cast `PlayerGameController` (`self.GetController` _asdimention_character)))
  (`PlayerController.SetViewTargetWithBlend` _asplayer_game_controller self 2.0 "VTBlend_Linear" 0.0 false)
  (`KismetSystemLibrary.Delay` 2.0)
  (`Controller.Possess` _asplayer_game_controller self)
  (`self.K2_DestroyActor` _asdimention_character))

(event `self.Sphere.OnComponentEndOverlap`
  (params (OverlappedComponent :type "PrimitiveComponent Object Reference") (OtherActor :type "Actor Object Reference") (OtherComp :type "PrimitiveComponent Object Reference") (OtherBodyIndex :type Integer)))

(event `InputAxis|MoveRight`
  (params (AxisValue :type "Float (single-precision)"))
  (`self.AddMovementInput` (* (`KismetMathLibrary.GetForwardVector` (`KismetMathLibrary.MakeRotator` 0.0 0.0 (.yaw (`self.GetControlRotation`)))) AxisValue)))

(event `InputAxis|LookUp`
  (params (AxisValue :type "Float (single-precision)")))

(event `InputAxis|Turn`
  (params (AxisValue :type "Float (single-precision)")))

(event `InputAction|Jump`
  (params (Key :type "Key Structure"))
  (bind _charactermovement (`self.CharacterMovement`))
  (:`Pressed`
    (if (> (`KismetMathLibrary.VSize` (`MovementComponent.Velocity` (`self.CharacterMovement`))) 0.0)
      (`self.Jump`)
      (set `CharacterMovementComponent.JumpZVelocity` 480.0 _charactermovement)
      (set `self.JumpPressed` true)
      (else
        (`self.Jump`)
        (set `CharacterMovementComponent.JumpZVelocity` 440.0 _charactermovement)
        (set `self.JumpPressed` true))))
  (:`Released`
    (set `self.JumpPressed` false)))

(event `InputAction|Interact`
  (params (Key :type "Key Structure"))
  (:`Pressed`
    (if (`KismetSystemLibrary.IsValid` (`self.TargetActor`))
      (bind _asplayer_game_controller (cast `PlayerGameController` (`self.GetController`)))
      (`InteractingActor.Interact` (`self.TargetActor`) _asplayer_game_controller))))

(fn `UserConstructionScript`)