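; BP_UpDownCube is a test actor whose cube starts or stops spinning each time it is acted on.
; BeginPlay binds a handler to OnAct, which flips IsActing and prints a debug string.
; While IsActing is set, Tick adds a small fixed local rotation to MainCube, unscaled by delta time.
; Despite its name, the graph contains no up-down movement.
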(event `self.ReceiveBeginPlay`
  (add `self.OnAct` (delegate `OnAct_Event_0`)))

(event `OnAct_Event_0`
  (set `self.IsActing` (not (`self.IsActing`)))
  (`KismetSystemLibrary.PrintString` "Acted"))

(event `self.ReceiveTick`
  (params (DeltaSeconds :type "Float (single-precision)"))
  (if (`self.IsActing`)
    (`SceneComponent.K2_AddLocalRotation` (`self.MainCube`) (struct :`Yaw` 0.1) false false)))

(fn `UserConstructionScript`)