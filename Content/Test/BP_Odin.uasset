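; BP_Odin is an interactable rotating puzzle piece that steps through a set number of yaw states toward a target state.
; Construction sets its starting yaw from the current state.
; Each interaction advances the state cyclically unless already rotating, and Tick then turns the actor incrementally by one step.
; When a finished step matches the target, it disables further rotation and notifies its Manager.
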(event `self.ReceiveBeginPlay`
  (add `InteractingActor.OnInteract` (delegate `OnInteract_Event_0`)))

(event `OnInteract_Event_0`
  (params (PlayerController :type "PlayerGameController Object Reference"))
  (`self.ChangeState`))

(event `self.ReceiveTick`
  (params (DeltaSeconds :type "Float (single-precision)"))
  (if (`self.Enabled`)
    (`self.Rotate` (* DeltaSeconds (`self.RotateVelocity`)))))

(fn `ChangeState`
  (if (not (`self.isRotating`))
    (set `self.State` (+ (mod (`self.State`) (`self.Number of states`)) 1))
    (set `self.Rotated` 0.0)
    (set `self.isRotating` true)))

(fn `Rotate`
  (params (RotationVelocity :type "Float (double-precision)"))
  (if (< (`self.Rotated`) (/ 360.0 (`KismetMathLibrary.Conv_IntToDouble` (`self.Number of states`))))
    (`self.K2_AddActorLocalRotation` (`KismetMathLibrary.MakeRotator` 0.0 0.0 RotationVelocity))
    (set `self.Rotated` (+ RotationVelocity (`self.Rotated`)))
    (else
      (set `self.isRotating` false)
      (if (== (`self.State`) (`self.TargetState`))
        (set `self.Enabled` false)
        (if (`KismetSystemLibrary.IsValid` (`self.Manager`))
          (`ActorManager.UpdateManager` (`self.Manager`)))))))

(fn `UserConstructionScript`
  (`self.K2_SetActorRotation` (`KismetMathLibrary.MakeRotator` 0.0 0.0 (+ (* (`KismetMathLibrary.Conv_IntToDouble` (`self.State`)) (/ 360.0 (`KismetMathLibrary.Conv_IntToDouble` (`self.Number of states`)))) 1.0 -180.0))))