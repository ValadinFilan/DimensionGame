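; BP_Stairs assembles tagged actors from the level into an animated staircase.
; BeginPlay records their transforms, shuffles them and assigns alternating left/right end slots in pairs, stepping by OffsetX and OffsetZ from the actor's location.
; The OnAct event starts a timeline that lerps each actor from original to slot transform, then calls FloatMessage on each.
; Float and StopFloat set and return FloatBOOL.
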(event `self.ReceiveBeginPlay`
  (bind _returnvalue (`self.K2_GetActorLocation`))
  (bind _stairsarray (`self.StairsArray`))
  (bind _stairsarray_2 (`self.StairsArray`))
  (bind _num (`self.num`))
  (bind _returnvalue_2 (* _num (`self.OffsetZ`)))
  (bind _returnvalue_3 (* _num (`self.OffsetX`)))
  ;[1 1 1] Setting Array
  (for _array_element (`self.Actor Class`)
    (bind _outactors (`GameplayStatics.GetAllActorsOfClassWithTag` _array_element (`self.TagToGet`)))
    (for _array_element_2 _outactors
      (`KismetArrayLibrary.Array_Add` (`self.StairsArray`) (make `/Game/Actors/Stairs/Stair` "0.000000,0.000000,0.000000|0.000000,0.000000,0.000000|1.000000,1.000000,1.000000" (`self.GetTransform` _array_element_2) _array_element_2))))
  ;[1 1 1] Randomize Elements
  (add `self.OnAct` (delegate `StartAnimation`))
  (`KismetArrayLibrary.Array_Shuffle` _stairsarray)
  (for (_array_element_3 _array_index) _stairsarray
    (`/Engine/EditorBlueprintResources/StandardMacros.FlipFlop`
      (:`A`
        (bind (_end _begin _stair) (break `/Game/Actors/Stairs/Stair` _array_element_3))
        (`KismetArrayLibrary.Array_Set` _stairsarray_2 _array_index (make `/Game/Actors/Stairs/Stair` (`KismetMathLibrary.MakeTransform` (+ (`KismetMathLibrary.MakeVector` _returnvalue_3 40.0 _returnvalue_2) _returnvalue) (struct) (20.0 20.0 20.0)) _begin _stair)))
      (:`B`
        (`KismetArrayLibrary.Array_Set` _stairsarray_2 _array_index (make `/Game/Actors/Stairs/Stair` (`KismetMathLibrary.MakeTransform` (+ (`KismetMathLibrary.MakeVector` _returnvalue_3 -40.0 _returnvalue_2) _returnvalue) (struct) (20.0 20.0 20.0)) _begin _stair))
        (set `self.num` (+ (`self.num`) 1))))))

(event `StartAnimation`
  (bind _stairsarray (`self.StairsArray`))
  ;[1 1 1] Animation
  (bind (_direction _newtrack_0) (`Timeline|Animation`)
    (:`Update`
      (for _array_element _stairsarray
        (bind (_end _begin _stair) (break `/Game/Actors/Stairs/Stair` _array_element))
        (`self.K2_SetActorTransform` _stair (`KismetMathLibrary.TLerp` _begin _end _newtrack_0 "EulerInterp") false false)))
    (:`Finished`
      (for _array_element_2 _stairsarray
        (message `/Game/Actors/Stairs/StairInterface.Float` (`.Stair_7_F4A60D6E4DA78E8DE39DC5826B94CB2B` (break `/Game/Actors/Stairs/Stair` _array_element_2)))))))

(fn `Float`
  (returns (float :type Boolean))
  (bind _output_get (set `self.floatBOOL` true))
  (return _output_get))

(fn `StopFloat`
  (returns (Float :type Boolean))
  (bind _output_get (set `self.floatBOOL` false))
  (return _output_get))

(fn `UserConstructionScript`)